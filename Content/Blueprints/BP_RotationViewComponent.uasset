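; Actor component that lets the player spin its owning actor by dragging with a touch, with inertial coasting after release.
; Each tick it turns the clamped Touch1 movement into X/Y scroll velocities, which drive world yaw and pitch scaled by RotateSpeed.
; On release, velocities decay toward zero through proportional friction plus constant drag, without reversing.
; Touch state changes only re-cache the position, avoiding jumps.
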(event EventBeginPlay)

(event EventTick
  (params (DeltaSeconds :type Float%20%28single-precision%29))
  (if (!= (Variables|Default|GetIsTouching) (.bIsCurrentlyPressed (Class|PlayerController|GetInputTouchState (Game|GetPlayerController 0) "Touch1")))
    (CallFunction|CacheTouchState)
    (else
      (CallFunction|CalcScrollVelecity DeltaSeconds)
      (CallFunction|RotateOwnerActor (* (Variables|Default|GetScrollVelocityX) DeltaSeconds) (* (Variables|Default|GetScrollVelocityY) DeltaSeconds)))))

(fn RotateOwnerActor
  (params (DeltaX :type Float%20%28double-precision%29) (DeltaY :type Float%20%28double-precision%29))
  (bind _rotatespeed (Variables|Default|GetRotateSpeed))
  (Class|Actor|AddActorWorldRotation (Components|GetOwner) (Math|Rotator|MakeRotator 0.0 (* DeltaY _rotatespeed) (* DeltaX _rotatespeed -1.0))))

(fn UpdateScrollInertialVelecity
  (params (DeltaSconds :type Float%20%28double-precision%29) (InSpeed :type Float%20%28double-precision%29))
  (bind _returnvalue (> InSpeed 0.0))
  (bind _frictioncoefficient (Variables|Default|GetFrictionCoefficient))
  (bind _staticvelocitydrag (Variables|Default|GetStaticVelocityDrag))
  (bind _returnvalue_2 (* _frictioncoefficient InSpeed DeltaSconds))
  (bind _returnvalue_3 (* _staticvelocitydrag -1.0))
  (bind _returnvalue_4 (Math|Float|SelectFloat _staticvelocitydrag _returnvalue_3 _returnvalue))
  (bind _returnvalue_5 (* DeltaSconds _returnvalue_4))
  (bind _returnvalue_6 (+ _returnvalue_2 _returnvalue_5))
  (bind _returnvalue_7 (- InSpeed _returnvalue_6))
  (return (Math|Float|SelectFloat (Math|Float|Max(Float) 0.0 _returnvalue_7) (Math|Float|Min(Float) 0.0 _returnvalue_7) _returnvalue)))

(fn CalcScrollVelecity
  (params (DeltaSeconds :type Float%20%28double-precision%29))
  (bind _returnvalue (Game|GetPlayerController 0))
  (bind (_locationx _locationy _biscurrentlypressed) (Class|PlayerController|GetInputTouchState _returnvalue "Touch1"))
  (if _biscurrentlypressed
    (Variables|Default|SetScrollVelocityX (/ (Math|Float|Clamp(Float) (- _locationx (Variables|Default|GetTouchPosX)) -25.0 25.0) DeltaSeconds))
    (Variables|Default|SetScrollVelocityY (/ (Math|Float|Clamp(Float) (- _locationy (Variables|Default|GetTouchPosY)) -25.0 25.0) DeltaSeconds))
    (CallFunction|CacheTouchState)
    (else
      ;[1 1 1] stop touch
      (Utilities|FlowControl|Sequence
        (:then_0
          (if (!= (Variables|Default|GetScrollVelocityX) 0.0) ; Inertial rotating  鼠标惯性
            (Variables|Default|SetScrollVelocityX (CallFunction|UpdateScrollInertialVelecity DeltaSeconds (Variables|Default|GetScrollVelocityX)))))
        (:then_1
          (if (!= (Variables|Default|GetScrollVelocityY) 0.0) ; Inertial rotating  鼠标惯性
            (Variables|Default|SetScrollVelocityY (CallFunction|UpdateScrollInertialVelecity DeltaSeconds (Variables|Default|GetScrollVelocityY)))))))))

(fn CacheTouchState
  (bind _returnvalue (Game|GetPlayerController 0))
  (bind (_locationx _locationy _biscurrentlypressed) (Class|PlayerController|GetInputTouchState _returnvalue "Touch1"))
  (Variables|Default|SetIsTouching _biscurrentlypressed)
  (Variables|Default|SetTouchPosX _locationx)
  (Variables|Default|SetTouchPosY _locationy))